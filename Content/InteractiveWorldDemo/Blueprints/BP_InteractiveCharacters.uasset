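; Character Blueprint for the Interactive World demo that makes movement slower and more sluggish on snow.
; A looping timer started at BeginPlay runs a short downward object trace against WorldStatic from the mesh location, instead of using Tick.
; When the hit physical material is PM_Snow it lowers max walk speed and acceleration on the movement component, otherwise it sets the faster values.
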(event Custom|CustomEvent
  (bind _charactermovement (Variables|Character|GetCharacterMovement))
  (bind _mesh (Variables|Character|GetMesh))
  (bind _returnvalue (Transformation|GetWorldLocation _mesh))
  (bind _outhit (Collision|LineTraceForObjects (+ _returnvalue "0,0,20.000000") (+ _returnvalue "0,0,-50.000000") (Utilities|Array|MakeArray "ObjectTypeQuery1") false 0 "None"))
  (if (== (.PhysMat (Collision|BreakHitResult _outhit)) "/Game/InteractiveWorldDemo/Map/WorldDemo/PhysicalMaterial/PM_Snow.PM_Snow")
    (Variables|/Script/Engine.CharacterMovementComponent|SetMaxWalkSpeed _charactermovement 4e+02)
    (Variables|/Script/Engine.CharacterMovementComponent|SetMaxAcceleration _charactermovement 2e+02)
    (else
      (Variables|/Script/Engine.CharacterMovementComponent|SetMaxWalkSpeed _charactermovement 6e+02)
      (Variables|/Script/Engine.CharacterMovementComponent|SetMaxAcceleration _charactermovement 1.5e+03))))

(event EventBeginPlay
  (Utilities|Time|SetTimerbyEvent (delegate Custom|CustomEvent) 0.05 true false -0.049))

(event Collision|EventActorBeginOverlap
  (params (OtherActor :type Actor%20Object%20Reference)))

(event EventTick
  (params (DeltaSeconds :type Float%20%28single-precision%29)))

(fn ConstructionScript
  (|CallParentFunction))